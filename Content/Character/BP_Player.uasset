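; BP_Player is the player character Blueprint, holding what looks like debug logic for flashlight enemies.
; Pressing X with authority finds every FlashlightEnemy and flips the Hunting bool on each one's Blackboard.
; An unconnected fragment would print the FlashlightComponent's current hit enemy, and the Tick and construction script are empty.
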(event EventBeginPlay)

(event Collision|EventActorBeginOverlap
  (params (OtherActor :type Actor%20Object%20Reference)))

(event EventTick
  (params (DeltaSeconds :type Float%20%28single-precision%29)))

(event Input|KeyboardEvents|X
  (params (Key :type Key%20Structure :default "None"))
  (bind _returnvalue (Utilities|Name|MakeLiteralName "Hunting"))
  (:Pressed
    (if (Ability|HasAuthority)
      (bind _outactors (Actor|GetAllActorsOfClass "/Script/FlashlightFrequency.FlashlightEnemy"))
      (for _array_element _outactors
        (AI|Components|Blackboard|SetValueasBool (AI|GetBlackboard _array_element) _returnvalue (not (ScalableFloat|GetValueasBool (AI|GetBlackboard _array_element) _returnvalue)))))))

(fn ConstructionScript)